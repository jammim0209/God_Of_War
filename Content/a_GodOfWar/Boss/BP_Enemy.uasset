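; Boss enemy Blueprint that loads its health and attack from the "Baldur" row of DT_StatusTable and caches its AI controller on BeginPlay.
; OnHit calls OnDamaged, currently with zero damage, prints health, then sets a new behavior state on AIC_Enemy and triggers its state change.
; Left-hand collision hits only print the other actor's path, and the loaded attack value is not used here.
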(event `self.ReceiveBeginPlay`
  (set `self.EnemyAIController` (`AIBlueprintHelperLibrary.GetAIController` self))
  (bind _returnvalue (`|GetDataTableRow` "/Game/a_GodOfWar/Boss/AI/DT_StatusTable.DT_StatusTable" "Baldur")
    (:`then`
      (set `self.HealthPoint` (break `/Game/a_GodOfWar/Boss/AI/S_Status` _returnvalue))
      (set `self.Attack` (`.Attack_5_6BEF411C4F42692D21C0BCA78AF92DE9` (break `/Game/a_GodOfWar/Boss/AI/S_Status` _returnvalue))))))

(event `self.LeftHand Collision.OnComponentHit`
  (params (HitComponent :type "PrimitiveComponent Object Reference") (OtherActor :type "Actor Object Reference") (OtherComp :type "PrimitiveComponent Object Reference") (NormalImpulse :type "Vector Structure") (Hit :type "HitResult Structure (by ref)"))
  (`KismetSystemLibrary.PrintString` (`KismetSystemLibrary.GetPathName` OtherActor)))

(fn `OnDamaged`
  (params (InDamage :type "Float (double-precision)"))
  (set `self.HealthPoint` (- (`self.HealthPoint`) InDamage)))

(fn `OnHit`
  ; 데미지를 입고
  (`self.OnDamaged` 0.0)
  (`KismetSystemLibrary.PrintString` (`KismetStringLibrary.Conv_DoubleToString` (`self.HealthPoint`)))
  (bind _asaic_enemy (cast `/Game/a_GodOfWar/Boss/AIC_Enemy` (`AIBlueprintHelperLibrary.GetAIController` self)))
  (set `/Game/a_GodOfWar/Boss/AIC_Enemy.BehaviorState` "NewEnumerator3" _asaic_enemy)
  (`/Game/a_GodOfWar/Boss/AIC_Enemy.ChangeState` _asaic_enemy))

(fn `UserConstructionScript`)