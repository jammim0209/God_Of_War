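; BP_GodOFWar is the UI manager for a God of War-style game, creating the health, quest, game-over and clear widgets.
; BeginPlay adds the HP bar and quest widget.
; Health updates route BP_Enemy to Baldur's bar and others to Kratos's, while a second update event always targets Kratos's.
; BP_DIE hides the HP UI and switches to cursor-driven UI-only input on the game-over screen; BP_Clear calls HPUI.Boss and shows the clear screen.
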(event `self.ReceiveTick`
  (params (DeltaSeconds :type "Float (single-precision)"))
  (bind _asbp_worldmove (cast `/Game/a_GodOfWar/BLUE_P/BP_worldmove` (`self.GetOwner`)))
  (set `self.As BP Worldmove` _asbp_worldmove))

(event `self.ReceiveBeginPlay`
  (`self.player_Hpbar`)
  (`self.Quest` false))

(event `BP_DIE`
  (params (IsGameove :type Boolean :default true))
  (`self.Gameover_state` IsGameove))

(event `BP_Clear`
  (params (`IsClear?` :type Boolean))
  (`/Game/a_GodOfWar/UI/WBP_HPbar.boss` (`self.HPUI`))
  (`self.Clear` `IsClear?`))

(event `BP_Quest`
  (params (`on?` :type Boolean)))

(event `UpdateHpBar`
  (params (CharacterObject :type "Actor Object Reference") (CurrentHp :type "Float (double-precision)") (MaxHp :type "Float (double-precision)"))
  (bind _hpui (`self.HPUI`))
  (cast `/Game/a_GodOfWar/Boss/BP_Enemy` CharacterObject
    (:`then`
      (`/Game/a_GodOfWar/UI/WBP_HPbar.UpdateBaldurHealth` _hpui CurrentHp MaxHp))
    (:`CastFailed`
      (`/Game/a_GodOfWar/UI/WBP_HPbar.UpdateKretosHealth` _hpui CurrentHp MaxHp))))

(event `Update_Hpbar`
  (params (CharacterObject :type "Actor Object Reference") (CurrentHp :type "Float (double-precision)") (MaxHp :type "Float (double-precision)"))
  (`/Game/a_GodOfWar/UI/WBP_HPbar.UpdateKretosHealth` (`self.HPUI`) CurrentHp MaxHp))

(fn `Clear`
  (params (`IsClear?` :type Boolean) (Event :type Delegate) (Event1 :type Delegate))
  (set `self.IsClear?` `IsClear?`)
  (bind _returnvalue (`|CreateWidget` "/Game/a_GodOfWar/UI/WBP_clear.WBP_clear_C"))
  (bind _output_get (set `self.ClearUi` _returnvalue))
  (`UserWidget.AddToViewport` _output_get 0))

(fn `Gameover_state`
  (params (`IsGameover?` :type Boolean))
  (bind _returnvalue (`GameplayStatics.GetPlayerController` 0))
  (set `self.IsGameover?` `IsGameover?`)
  (bind _returnvalue_2 (`|CreateWidget` "/Game/a_GodOfWar/UI/GameOver.GameOver_C"))
  (bind _output_get (set `self.OVERui` _returnvalue_2))
  (`UserWidget.AddToViewport` (`self.OVERui`) 1)
  (`UserWidget.AddToViewport` _output_get 1)
  (set `Widget.Visibility` "Hidden" (`self.HPUI`))
  (set `PlayerController.bShowMouseCursor` true _returnvalue)
  (`WidgetBlueprintLibrary.SetInputMode_UIOnlyEx` _returnvalue null))

(fn `player_Hpbar`
  (`/Engine/EditorBlueprintResources/StandardMacros.IsValid` (`self.HPUI`)
    (:`Is Valid`
      (bind _returnvalue (`|CreateWidget` "/Game/a_GodOfWar/UI/WBP_HPbar1.WBP_HPbar1_C"))
      (bind _output_get (set `self.NewVar` _returnvalue))
      (`UserWidget.AddToViewport` _output_get 0))
    (:`Is Not Valid`
      (bind _returnvalue_2 (`|CreateWidget` "/Game/a_GodOfWar/UI/WBP_HPbar.WBP_HPbar_C"))
      (bind _output_get_2 (set `self.HPUI` _returnvalue_2))
      (`UserWidget.AddToViewport` _output_get_2 0))))

(fn `Quest`
  (params (`on?` :type Boolean))
  (set `self.on?` `on?`)
  (bind _returnvalue (`|CreateWidget` "/Game/a_GodOfWar/UI/Quest.Quest_C"))
  (bind _output_get (set `self.NewVar_0` _returnvalue))
  (`UserWidget.AddToViewport` _output_get 0))

(fn `UserConstructionScript`)