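; Actor component that tracks health and death state for whatever owns it.
; On BeginPlay it sets current health to the maximum.
; Increase and decrease functions adjust health, capping it at the maximum and flooring it at zero.
; The death flag is set and returned only when damage pushes health below zero, so landing exactly on zero does not set it.
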(event `self.ReceiveBeginPlay`
  (`self.initializeStat`))

(fn `decressHealth`
  (params (DamagePoint :type "Float (double-precision)"))
  (returns (IsDead :type Boolean))
  ; current Health 가 0 미만이면 0으로 고정
  (set `self.currentHealth` (- (`self.currentHealth`) DamagePoint))
  (if (< (`self.currentHealth`) 0.0)
    (set `self.currentHealth` 0.0)
    (bind _output_get (set `self.IsDead?` true))
    (return _output_get)))

(fn `incressHealth`
  (params (healthpoint :type "Float (double-precision)"))
  ; 현재 체력이 최대로 넘어가면 최대 체력으로 설정
  (set `self.currentHealth` (+ healthpoint (`self.currentHealth`)))
  (if (> (`self.currentHealth`) (`self.Maxheath`))
    (set `self.currentHealth` (`self.Maxheath`))))

(fn `initializeStat`
  (set `self.currentHealth` (`self.Maxheath`)))