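; Actor component for the third-person character that runs a melee attack combo from the IA_Attack input.
; An Attack flag gates input, and Combocount selects which montage plays on the character mesh.
; Notify Begin advances the first three stages and clears the gate, though the first also clears it immediately; the fourth reuses the second montage and resets only on interruption.
; These paths set a one-second timer that zeroes the count.
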(event `self.ReceiveBeginPlay`
  (bind _asbp_third_person_character (cast `/Game/a_GodOfWar/third_Person/BP_ThirdPersonCharacter` (`self.GetOwner`)))
  (bind _output_get (set `self.As BP Third Person Character` _asbp_third_person_character))
  (set `self.charactermesh` (`Character.Mesh` _output_get)))

(event `EnhancedInput|/Game/Input/Actions/IA_Attack`
  (params (ActionValue :type Boolean) (ElapsedSeconds :type "Float (double-precision)") (TriggeredSeconds :type "Float (double-precision)") (InputAction :type "InputAction Object Reference" :default "/Game/Input/Actions/IA_Attack.IA_Attack"))
  (bind _charactermesh (`self.charactermesh`))
  (:`Started`
    (if (not (`self.attack`))
      (set `self.attack` true) ; attack가false일떄만작용됌
      (switch `int` (`self.combocount`)
        (:`0`
          (`|PlayMontage` _charactermesh "/Game/a_GodOfWar/anim/montage/a_one_montage.a_one_montage"
            (:`then`
              _)
            (:`OnNotifyBegin`
              (set `self.attack` false)
              (set `self.combocount` 1))))
        (:`1`
          (`|PlayMontage` _charactermesh "/Game/a_GodOfWar/anim/montage/a_two_montage.a_two_montage"
            (:`OnNotifyBegin`
              (set `self.attack` false)
              (set `self.combocount` 2))))
        (:`2`
          (`|PlayMontage` _charactermesh "/Game/a_GodOfWar/anim/montage/a_three_montage.a_three_montage"
            (:`OnNotifyBegin`
              (set `self.attack` false)
              (set `self.combocount` 3))))
        (:`3`
          (`|PlayMontage` _charactermesh "/Game/a_GodOfWar/anim/montage/a_two_montage.a_two_montage"
            (:`OnInterrupted`
              (set `self.attack` false)
              (set `self.combocount` 0)))))
      (`KismetSystemLibrary.K2_SetTimerDelegate` (delegate `resetcounter`) 1.0)
      (set `self.attack` false))))

(event `resetcounter`
  (set `self.combocount` 0))