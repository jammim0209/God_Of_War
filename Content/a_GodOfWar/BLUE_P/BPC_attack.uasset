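; BPC_attack is an attack component for the BP_kretos character, currently holding an early ranged-aim test.
; On BeginPlay it casts its owner to BP_kretos and caches that reference and its mesh.
; The firerange event line-traces on the Visibility channel forward from the CameraBoom to aim from the camera, with debug drawing.
; The trace result is not used yet, so no damage or projectile follows.
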(event `self.ReceiveBeginPlay`
  (bind _asbp_kretos (cast `/Game/a_GodOfWar/third_Person/BP_kretos` (`self.GetOwner`)))
  (bind _output_get (set `self.As BP Kretos` _asbp_kretos))
  (set `self.character_skm` (`Character.Mesh` _output_get)))

(event `firerange`
  (bind _cameraboom (`/Game/a_GodOfWar/third_Person/BP_kretos.CameraBoom` (`self.As BP Kretos`)))
  (bind _returnvalue (`SceneComponent.K2_GetComponentLocation` _cameraboom))
  ; 카메라에서 조준
  (`KismetSystemLibrary.LineTraceSingle` :`Start` _returnvalue :`End` (+ _returnvalue (* (`SceneComponent.GetForwardVector` _cameraboom) 2000.0)) :`TraceChannel` "TraceTypeQuery1" :`DrawDebugType` "ForDuration"))