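; Axe weapon actor that deals damage through sphere traces, spins and destroys itself on impact.
; Every tick, its attack trace component traces at the collision component's location, with identical start and end since no socket is named, passing base damage and itself as causer.
; Static mesh activation sets the rotating movement's spin rate, and a mesh hit destroys the actor after a short delay.
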(event `self.ReceiveTick`
  (params (DeltaSeconds :type "Float (single-precision)"))
  (bind _collison (`self.collison`))
  (`/Game/a_GodOfWar/BLUE_P/BPC_attacktrace.attacksphereTracce` (`self.BPC_attacktrace`) (`SceneComponent.GetSocketLocation` _collison "None") (`SceneComponent.GetSocketLocation` _collison "None") (`self.Base Damage`) self))

(event `self.StaticMesh.OnComponentActivated`
  (params (Component :type "ActorComponent Object Reference") (bReset :type Boolean))
  (set `RotatingMovementComponent.RotationRate` (`KismetMathLibrary.MakeRotator` 180.0 90.0 90.0) (`self.RotatingMovement`)))

(event `self.StaticMesh.OnComponentHit`
  (params (HitComponent :type "PrimitiveComponent Object Reference") (OtherActor :type "Actor Object Reference") (OtherComp :type "PrimitiveComponent Object Reference") (NormalImpulse :type "Vector Structure") (Hit :type "HitResult Structure (by ref)"))
  (`KismetSystemLibrary.Delay` 0.2)
  (`self.K2_DestroyActor`))

(fn `UserConstructionScript`)