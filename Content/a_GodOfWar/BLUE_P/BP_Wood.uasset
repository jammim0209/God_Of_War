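; BP_Wood is a damageable wood actor that bursts apart when hit.
; Any damage is passed to its BPCTreeHP component, then fires a radial force impulse and spawns an explosion emitter at the location from the Wood mesh's hit event.
; The actor is destroyed after a short delay regardless of remaining HP, so the later death check is redundant.
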(event `self.ReceiveAnyDamage`
  (params (Damage :type "Float (single-precision)") (DamageType :type "DamageType Object Reference") (InstigatedBy :type "Controller Object Reference") (DamageCauser :type "Actor Object Reference"))
  (set `self.Damage Causer_0` DamageCauser)
  (bind _newparam (`/Game/a_GodOfWar/BLUE_P/BPC_treeHP.decress` (`self.BPC_treeHP`) Damage))
  (`RadialForceComponent.FireImpulse` (`self.RadialForce`))
  (`GameplayStatics.SpawnEmitterAtLocation` "/Game/StarterContent/Particles/P_Explosion.P_Explosion" (`.Location` (`GameplayStatics.BreakHitResult` (stale `self.wood.OnComponentHit` Hit))))
  (`KismetSystemLibrary.Delay` 0.2)
  (`self.K2_DestroyActor`)
  (bind _output_get (set `self.Is Dead` _newparam))
  (if _output_get
    (`self.K2_DestroyActor`)))

(event `self.wood.OnComponentHit`
  (params (HitComponent :type "PrimitiveComponent Object Reference") (OtherActor :type "Actor Object Reference") (OtherComp :type "PrimitiveComponent Object Reference") (NormalImpulse :type "Vector Structure") (Hit :type "HitResult Structure (by ref)")))

(fn `UserConstructionScript`)