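; BP_GameWhill is an actor that removes its StaticMesh1 component seven seconds after something begins overlapping its Box.
; NewFunction forwards an HP value to BPCTreeHP's Decress and branches on the result, but nothing follows the branch.
; A component-destroy and attached explosion emitter sit unconnected and never run, and the Box click event is empty.
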(event `self.Box.OnComponentBeginOverlap`
  (params (OverlappedComponent :type "PrimitiveComponent Object Reference") (OtherActor :type "Actor Object Reference") (OtherComp :type "PrimitiveComponent Object Reference") (OtherBodyIndex :type Integer) (bFromSweep :type Boolean) (SweepResult :type "HitResult Structure (by ref)"))
  (`KismetSystemLibrary.Delay` 7.0)
  (`ActorComponent.K2_DestroyComponent` (`self.StaticMesh1`)))

(event `self.Box.OnClicked`
  (params (TouchedComponent :type "PrimitiveComponent Object Reference") (ButtonPressed :type "Key Structure")))

(fn `NewFunction`
  (params (HP :type "Float (double-precision)" :default 1.0) (`Damage Causer` :type "Actor Object Reference"))
  (set `self.Damage Causer` `Damage Causer`)
  (bind _newparam (`/Game/a_GodOfWar/BLUE_P/BPC_treeHP.decress` (`self.BPC_treeHP`) HP))
  (if _newparam
    _))

(fn `UserConstructionScript`)