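; BP_GameWall is a destructible wall that explodes and dissolves when a BP_axe overlaps its trigger sphere.
; The hit disables the sphere's collision, then after short delays destroys the WHill component and plays explosion, smoke and rock effects.
; A death flag lets Tick raise a scalar on the dynamic dissolve material each frame, and a delay then destroys the static mesh.
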(event `self.Sphere.OnComponentBeginOverlap`
  (params (OverlappedComponent :type "PrimitiveComponent Object Reference") (OtherActor :type "Actor Object Reference") (OtherComp :type "PrimitiveComponent Object Reference") (OtherBodyIndex :type Integer) (bFromSweep :type Boolean) (SweepResult :type "HitResult Structure (by ref)"))
  (bind _asbp_axe (cast `/Game/a_GodOfWar/BLUE_P/axe/BP_axe` OtherActor))
  (set `self.As BP Axe` _asbp_axe)
  (`PrimitiveComponent.SetCollisionEnabled` (`self.Sphere`) "NoCollision")
  (`/Engine/EditorBlueprintResources/StandardMacros.IsValid` (`self.wHill`)
    (:`Is Valid`
      (`KismetSystemLibrary.Delay` 0.2)
      (set `self.Is Dead_0` true)
      (`GameplayStatics.PlaySound2D` "/Game/StarterContent/Audio/Explosion01.Explosion01" 1.0 1.0 0.0 null null)
      (`ActorComponent.K2_DestroyComponent` (`self.wHill`))
      (`GameplayStatics.SpawnEmitterAttached` "/Game/StarterContent/Particles/P_Explosion.P_Explosion" (`self.particale`))
      (`KismetSystemLibrary.Delay` 1.0)
      (`GameplayStatics.SpawnEmitterAttached` "/Game/StarterContent/Particles/P_Smoke.P_Smoke" (`self.StaticMesh`))
      (`GameplayStatics.PlaySound2D` "/Game/StarterContent/Audio/Smoke01.Smoke01" 1.0 1.0 0.0 null null)
      (`GameplayStatics.PlaySound2D` "/Game/a_GodOfWar/sound/rock.rock" 1.0 1.0 0.0 null null)
      (set `self.CurDessovle` (+ (* (stale `self.ReceiveTick` DeltaSeconds) (`self.DessolveSpeed`)) (`self.CurDessovle`)) :!label _label)
      (`MaterialInstanceDynamic.SetScalarParameterValue` (`self.Mat`) "value" (`self.CurDessovle`))
      (`/Engine/EditorBlueprintResources/StandardMacros.IsValid` (`self.StaticMesh`)
        (:`Is Valid`
          (`KismetSystemLibrary.Delay` 3.5)
          (`ActorComponent.K2_DestroyComponent` (`self.StaticMesh`)))))))

(event `self.ReceiveBeginPlay`
  (bind _returnvalue (`PrimitiveComponent.CreateDynamicMaterialInstance` (`self.StaticMesh`) 0 "/Game/a_GodOfWar/object/Material/deslove_effect_Inst.deslove_effect_Inst" "None"))
  (bind _output_get (set `self.Mat` _returnvalue))
  (bind _returnvalue_2 (`MaterialInstanceDynamic.K2_GetScalarParameterValue` _output_get "value"))
  (set `self.CurDessovle` _returnvalue_2))

(event `self.ReceiveTick`
  (params (DeltaSeconds :type "Float (single-precision)"))
  (if (`self.Is Dead_0`)
    (goto _label)))

(fn `UserConstructionScript`)