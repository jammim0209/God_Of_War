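; Attack trace component for BP_kretos that applies melee damage from hand-based sphere traces.
; Starting an attack sets a non-looping 0.1-second timer for the trace, and stopping clears it.
; The trace sweeps from a hand component to an offset point on the Camera channel, with a constant selector always picking the right hand.
; Hits apply damage credited to the character, with debug drawing and a printed message.
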(event `self.ReceiveBeginPlay`
  ; casthing
  (bind _asbp_kretos (cast `/Game/a_GodOfWar/third_Person/BP_kretos` (`self.GetOwner`)))
  (bind _output_get (set `self.As BP Third Person Character` _asbp_kretos))
  (set `self.Mesh` (`Character.Mesh` _output_get)))

(event `startattackTrace`
  ; 피격 범위 설정(shpere 가 안보인다면trace channel , camera,  draw debug 에서 peresitent )
  (bind _returnvalue (`KismetSystemLibrary.K2_SetTimerDelegate` (delegate `AttackTrace`) 0.1))
  (set `self.attackTimerHandler` _returnvalue))

(event `AttackTrace`
  (bind _as_bp_third_person_character (`self.As BP Third Person Character`))
  (bind (_start _end) (`self.getHandLocation` (`/Game/a_GodOfWar/third_Person/BP_kretos.rightHand` _as_bp_third_person_character)))
  (bind (_start_2 _end_2) (`self.getHandLocation` (`/Game/a_GodOfWar/third_Person/BP_kretos.leftHand` _as_bp_third_person_character)))
  ; 피격 범위 설정(shpere 가 안보인다면trace channel , camera,  draw debug 에서 peresitent )
  (switch `int` 0
    (:`0`
      (`self.attacksphereTracce` _start _end (`self.Base Damage`) (`self.As BP Third Person Character`)))
    (:`1`
      (`self.attacksphereTracce` _start_2 _end_2 (`self.Base Damage`) (`self.As BP Third Person Character`)))))

(event `stopAttackTRace`
  ; 피격 범위 설정(shpere 가 안보인다면trace channel , camera,  draw debug 에서 peresitent )
  (`KismetSystemLibrary.K2_ClearAndInvalidateTimerHandle` (`self.attackTimerHandler`)))

(fn `attacksphereTracce`
  (params (Start :type "Vector Structure") (End :type "Vector Structure") (BaseDamage :type "Float (single-precision)") (DamageCauser :type "Actor Object Reference"))
  (bind (_outhit _returnvalue) (`KismetSystemLibrary.SphereTraceSingle` :`Start` Start :`End` End :`Radius` 20.0 :`TraceChannel` "TraceTypeQuery2" :`DrawDebugType` "ForDuration" :`DrawTime` 7.0))
  (if _returnvalue
    (`GameplayStatics.ApplyDamage` (`.HitActor` (`GameplayStatics.BreakHitResult` _outhit)) BaseDamage null DamageCauser)
    (`KismetSystemLibrary.PrintString` "attack!")))

(fn `getHandLocation`
  (params (hand :type "SceneComponent Object Reference"))
  (returns (start :type "Vector Structure") (end :type "Vector Structure"))
  (return (`SceneComponent.K2_GetComponentLocation` hand) (`KismetMathLibrary.TransformLocation` (`SceneComponent.K2_GetComponentToWorld` hand) (+ (`SceneComponent.RelativeLocation` hand) (20.0 0.0 0.0)))))