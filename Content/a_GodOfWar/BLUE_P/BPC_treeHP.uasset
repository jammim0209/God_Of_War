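; BPC_treeHP is a health component, apparently for trees, that tracks current HP against a maximum.
; It fills CurrentHP to MaxHP on BeginPlay and exposes functions to decrease or increase it, clamped at zero and MaxHP respectively.
; Decress sets and returns IsDead only when HP drops below zero, so landing exactly on zero does not flag death.
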(event `self.ReceiveBeginPlay`
  (`self.initializeStat`))

(fn `decress`
  (params (HP :type "Float (double-precision)"))
  (returns (NewParam :type Boolean))
  (set `self.currentHP` (- (`self.currentHP`) HP))
  (if (< (`self.currentHP`) 0.0)
    (set `self.currentHP` 0.0)
    (bind _output_get (set `self.IsDead` true))
    (return _output_get)))

(fn `incress`
  (params (HP :type "Float (double-precision)"))
  (set `self.currentHP` (+ HP (`self.currentHP`)))
  (if (> (`self.currentHP`) (`self.MaxHP`))
    (set `self.currentHP` (`self.MaxHP`))))

(fn `initializeStat`
  (set `self.currentHP` (`self.MaxHP`)))